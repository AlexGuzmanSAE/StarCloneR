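; Player actor that rides a spline track, shifts its mesh sideways and vertically from input, and fires darts.
; Tick advances it along SplineTrack, applies the offset, and interpolates mesh tilt, though GetVelocity currently returns zero.
; Holding left mouse runs a looping timer that redraws a predicted projectile path with spline meshes.
; Releasing clears the preview and launches a Dart_BP by camera-based impulse, computed separately from the preview velocity.
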(event Custom|Draw%20Path
  (bind _returnvalue (Utilities|Time|SetTimerbyEvent (delegate Custom|Update%20Curve) 0.01 true))
  (Variables|Default|SetProjectile%20Timer _returnvalue))

(event Custom|Update%20Curve
  (bind _returnvalue (Game|GetPlayerCameraManager 0))
  (bind _spline (Variables|Default|GetSpline))
  (bind _returnvalue_2 (Camera|GetCameraRotation _returnvalue))
  (bind _returnvalue_3 (Math|Vector|GetForwardVector _returnvalue_2))
  (bind _returnvalue_4 (* _returnvalue_3 1e+03))
  (bind (_x _y) (Math|Vector|BreakVector _returnvalue_4))
  (CallFunction|ClearSplinePoints)
  (bind _predictresult (Class|GameplayStatics|BlueprintPredictProjectilePathAdvanced (Utilities|Struct|MakePredictProjectilePathParams (Transformation|GetWorldLocation (Variables|Default|Getroot)) (Math|Vector|MakeVector _x _y (* (Math|Float|MapRangeUnclamped (.Z (Math|Vector|BreakVector _returnvalue_3)) 0.0 1.0 3.0 1e+01) 3e+04 0.0)) true 0.0 1.0 true "ECC_WorldStatic" "ObjectTypeQuery1" (Utilities|Array|MakeArray self) 2e+01 0.0 "None" 5.0 false)))
  (for _array_element (.PathData (Utilities|Struct|BreakPredictProjectilePathResult _predictresult))
    (Spline|AddSplinePoint (Variables|Default|GetSpline) (.Location (Utilities|Struct|BreakPredictProjectilePathPointData _array_element)) "World" true))
  (for _index (range 1 (Spline|GetNumberOfSplinePoints (Variables|Default|GetSpline)))
    (bind _returnvalue_5 (AddComponent|AddSplineMeshComponent true))
    (Utilities|Array|Add (Variables|Default|GetSplineMesh) _returnvalue_5)
    (SplineMesh|SetStartandEnd _returnvalue_5 (.Location (Spline|GetLocationandTangentatSplinePoint _spline _index "World")) (.Tangent (Spline|GetLocationandTangentatSplinePoint _spline _index "World")) (Math|Vector|Lerp(Vector) (.Location (Spline|GetLocationandTangentatSplinePoint _spline _index "World")) (.Location (Spline|GetLocationandTangentatSplinePoint _spline (+ _index 1) "World")) 0.5) (Math|Vector|Lerp(Vector) (.Tangent (Spline|GetLocationandTangentatSplinePoint _spline _index "World")) (.Tangent (Spline|GetLocationandTangentatSplinePoint _spline (+ _index 1) "World")) 0.5) true :!class /Script/Engine.SplineMeshComponent)))

(event Custom|Clear%20Spline%20Points
  (bind _splinemesh (Variables|Default|GetSplineMesh))
  (Components|DestroyComponent _splinemesh)
  (Utilities|Array|Clear _splinemesh)
  (Spline|ClearSplinePoints (Variables|Default|GetSpline) true))

(event EventTick
  (params (DeltaSeconds :type Float%20%28single-precision%29))
  (CallFunction|SnapSpline DeltaSeconds)
  (CallFunction|PlaneMove DeltaSeconds)
  (CallFunction|RotatewithSpline DeltaSeconds))

(event Input|MouseEvents|LeftMouseButton
  (params (Key :type Key%20Structure :default "None"))
  (bind _returnvalue (Game|GetPlayerCameraManager 0))
  (bind _returnvalue_2 (Camera|GetCameraRotation _returnvalue))
  (bind _returnvalue_3 (Math|Vector|GetForwardVector _returnvalue_2))
  (bind _returnvalue_4 (* _returnvalue_3 3e+03))
  (bind (_x _y) (Math|Vector|BreakVector _returnvalue_4))
  (:Pressed
    (CallFunction|DrawPath))
  (:Released
    (Utilities|Time|ClearandInvalidateTimerbyHandle (Variables|Default|GetProjectile%20Timer))
    (CallFunction|ClearSplinePoints)
    (bind _returnvalue_5 (Game|SpawnActorfromClass "/Game/NerfDart/Dart_BP.Dart_BP_C" (Math|Transform|MakeTransform (Transformation|GetWorldLocation (Variables|Default|Getroot)) "0, 0, 0" "1.000000,1.000000,1.000000") "Undefined" "MultiplyWithRoot" 0 0))
    (Physics|AddImpulse (Variables|/Game/NerfDart/Dart_BP.Dart_BP_C|GetDart _returnvalue_5) (Math|Vector|MakeVector _x _y (* (Math|Float|MapRangeUnclamped (.Z (Math|Vector|BreakVector _returnvalue_3)) 0.0 1.0 3.0 1e+01) 5e+02)) "None" false)
    (Transformation|SetActorRotation (Pawn|GetControlRotation :!class /Script/Engine.Pawn))
    (Development|PrintText "DARDO")))

(fn ConstructionScript)

(fn SnapSpline
  (params (deltaTime :type Float%20%28double-precision%29))
  (bind _output_get (Variables|Default|SetDistanceTraveled (+ (Variables|Default|GetDistanceTraveled) (* deltaTime (Variables|Default|GetSpeed)))))
  (bind _pivot (Default|GetPivotatDistance (Variables|Default|GetSpline%20Track) _output_get))
  (Transformation|SetActorTransform (Math|Transform|MakeTransform (.location _pivot) (.rotation _pivot) "1.000000,1.000000,1.000000")))

(fn PlaneMove
  (params (DeltaTime :type Float%20%28double-precision%29))
  (bind _output_get (Variables|Default|SetMovementSpeed (Math|Vector|MakeVector 0.0 (Input|AxisValues|GetInputHorizontal) (Input|AxisValues|GetInputVertical))))
  (bind _output_get_2 (Variables|Default|SetAdjusted%20Offset (+ (* (* _output_get (Variables|Default|GetSpeed)) DeltaTime) (Variables|Default|GetOffSet))))
  (bind _output_get_3 (Variables|Default|SetOffSet _output_get_2))
  (Math|Float|CompareFloat (.y _output_get_3) 0.0
    (:>
      _)
    (:<
      _))
  (Transformation|SetRelativeLocation (Variables|Character|GetMesh) (Math|Vector|MakeVector 0.0 (.y _output_get_3) (.z _output_get_3)) false false))

(fn Shoot)

(fn ManageParabola
  (bind _returnvalue (Utilities|Time|SetTimerbyFunctionName 0 "IncrementParabola" 0.0))
  (Variables|Default|SetTimer _returnvalue))

(fn ClearShootTimer
  (Utilities|Time|ClearandInvalidateTimerbyHandle (Variables|Default|GetTimer)))

(fn IncrementParabola)

(fn GetLocation
  (params (u :type Vector) (t :type Float%20%28double-precision%29))
  (return (+ (* u t) (Math|Vector|MakeVector 0.0 0.0 (* 0.5 -9.8e+02 t t)) (Transformation|GetWorldLocation (Variables|Default|GetRootSpline)))))

(fn RotatewithSpline
  (params (delta_time :type Float%20%28double-precision%29))
  (bind _mesh (Variables|Character|GetMesh))
  (bind _velocity (CallFunction|GetVelocity))
  (Transformation|SetRelativeRotation _mesh (Math|Interpolation|RInterpTo (Variables|/Script/Engine.SceneComponent|GetRelativeRotation _mesh) (Math|Rotator|MakeRotator (* (Math|Vector|DotProduct (Transformation|GetActorRightVector) (Math|Vector|Normalize _velocity)) 45.0) (* (Math|Vector|DotProduct (Math|Vector|Normalize _velocity) (Transformation|GetActorUpVector)) 3e+01) (* (Math|Vector|DotProduct (Transformation|GetActorRightVector) (Math|Vector|Normalize _velocity)) 15.0)) delta_time 0.0) false false))

(fn GetVelocity
  (bind _output_get (Variables|Default|SetMovementSpeed (Math|Vector|MakeVector (Input|AxisValues|GetInputHorizontal) (Input|AxisValues|GetInputVertical) 0.0)))
  (return "0, 0, 0"))

(event Custom|DrawTrayectory
  (params (start/stop :type Boolean))
  (bind _output_get (Variables|Default|SetDrawing start/stop))
  (if _output_get :!label _label
    (for _index (range 0 100)
      (bind _location (CallFunction|GetLocation (* (+ (Transformation|GetActorRightVector) "1.000000,0.000000,0.000000") 5e+02) (+ _index 0.01)))
      (Collision|LineTraceByChannel _location (+ _location "-10.000000,0.000000,-0.000000") "TraceTypeQuery2" false 0 "Persistent"))
    (Utilities|FlowControl|Delay 0.2)
    (goto _label)))